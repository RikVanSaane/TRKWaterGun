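; Water volume actor for the water gun: a placeable box of water with surface, underside and underwater post-process effects.
; InitBox stores its index and creates dynamic materials, passing the water height to the extinction and screen distortion blendables.
; SetBoxSize positions, yaws and scales the actor, matching material tiling to its size.
; RemoveBox, on authority only, asks TRKWaterGunSingleton to remove the instance by index; older level-unload code is disconnected.
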(event EventEndPlay
  (params (EndPlayReason :type EEndPlayReason%20Enum :default "ActorDestroyed"))
  ;[1 1 1] unload instance so it doesnt get saved, a new one is made from the spawner
)

(fn ConstructionScript)

(fn SetBoxSize
  (params (BoxSize :type Vector) (BoxPosition :type Vector) (BoxRotation :type Float%20%28single-precision%29))
  (bind _returnvalue (/ BoxSize 1.1811e+05))
  (bind (_x _y) (Math|Vector|BreakVector _returnvalue))
  (Transformation|SetActorTransform (Math|Transform|MakeTransform BoxPosition (Math|Rotator|MakeRotator 0.0 BoxRotation 0.0) (/ BoxSize 256.0)))
  (Rendering|Material|SetVectorParameterValue (Variables|Default|GetWaterMaterial) "TilingMult" (Utilities|Struct|MakeLinearColor _x _y 0.0 1.0) :!class /Script/Engine.MaterialInstanceDynamic)
  (Rendering|Material|SetVectorParameterValue (Variables|Default|GetWaterUndersideMaterial) "TilingMult" (Utilities|Struct|MakeLinearColor _x _y 0.0 1.0) :!class /Script/Engine.MaterialInstanceDynamic))

(fn InitBox
  (params (WaterHeight :type Float%20%28single-precision%29) (Index :type Integer))
  (bind _postprocess1 (Variables|Default|GetPostProcess1))
  (bind _settings (Variables|/Script/Engine.PostProcessComponent|GetSettings _postprocess1))
  (bind _blendables (Utilities|Struct|BreakPostProcessSettings _settings))
  (Variables|Default|SetThisIndex Index)
  (bind _returnvalue (Rendering|Material|CreateDynamicMaterialInstance "/Game/PrimalEarth/Environment/Water/Water_MatIsland_underside_MIC.Water_MatIsland_underside_MIC" :!class /Script/Engine.KismetMaterialLibrary))
  (Variables|Default|SetWaterUndersideMaterial _returnvalue)
  (Rendering|Material|SetMaterial (Variables|Default|GetStaticMesh2) 0 _returnvalue)
  (bind _returnvalue_2 (Rendering|Material|CreateDynamicMaterialInstance "/Game/PrimalEarth/Environment/Water/LakeWater_MatIsland_MIC.LakeWater_MatIsland_MIC" :!class /Script/Engine.KismetMaterialLibrary))
  (Variables|Default|SetWaterMaterial _returnvalue_2)
  (Rendering|Material|SetMaterial (Variables|Default|GetStaticMesh1) 0 _returnvalue_2)
  (bind _returnvalue_3 (Rendering|Material|CreateDynamicMaterialInstance "/Game/Mods/TRKWaterGun/WaterGun/Assets/PP_TRKunderwaterExtinction_Inst.PP_TRKunderwaterExtinction_Inst" :!class /Script/Engine.KismetMaterialLibrary))
  (Utilities|Array|SetArrayElem _blendables 0 _returnvalue_3)
  (Rendering|Material|SetScalarParameterValue _returnvalue_3 "TRKLocalWaterLevel" WaterHeight :!class /Script/Engine.MaterialInstanceDynamic)
  (bind _returnvalue_4 (Rendering|Material|CreateDynamicMaterialInstance "/Game/Mods/TRKWaterGun/WaterGun/Assets/PP_TRKwaterScreenDistortion_Inst.PP_TRKwaterScreenDistortion_Inst" :!class /Script/Engine.KismetMaterialLibrary))
  (Utilities|Array|SetArrayElem _blendables 1 _returnvalue_4)
  (Rendering|Material|SetScalarParameterValue _returnvalue_4 "TRKLocalWaterLevel" WaterHeight :!class /Script/Engine.MaterialInstanceDynamic))

(fn RemoveBox
  (Networking|SwitchHasAuthority
    (:Authority
      (bind _outactors (Actor|GetAllActorsOfClass "/Game/Mods/TRKWaterGun/WaterGun/TRKWaterGunSingleton.TRKWaterGunSingleton_C"))
      (bind _astrkwatergunsingleton_c (Utilities|Casting|CastToTRKWaterGunSingleton (Utilities|Array|Get(acopy) _outactors)))
      (Default|RemoveInstance _astrkwatergunsingleton_c (Variables|Default|GetThisIndex))
      (Development|PrintString "Removed Instance"))))