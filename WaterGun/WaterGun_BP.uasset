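; Water gun weapon for drawing, placing and removing box-shaped water volumes in the world.
; Three camera-traced shots define a rotated box via line-intersection math, previewed live by a spawned mesh.
; Right-click plus number keys then tune water level and depth before a fourth shot registers the volume with TRKWaterGunSingleton on authority.
; Right-click firing removes the targeted volume; an idle right-click+1+2 chord clears all spawners and singleton instances.
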(event Custom|DeleteAllVolumes
  ;[1 1 1] Deleting all objects from scene
  (Utilities|FlowControl|Sequence
    (:then_0
      (bind _outactors (Actor|GetAllActorsOfClass "/Game/Mods/TRKWaterGun/WaterGun/TRKVolumeSpawner.TRKVolumeSpawner_C"))
      (for _array_element _outactors
        (Actor|DestroyActor _array_element)))
    (:then_1
      (bind _outactors_2 (Actor|GetAllActorsOfClass "/Game/Mods/TRKWaterGun/WaterGun/TRKWaterGunSingleton.TRKWaterGunSingleton_C"))
      (bind _astrkwatergunsingleton_c (Utilities|Casting|CastToTRKWaterGunSingleton (Utilities|Array|Get(acopy) _outactors_2)))
      (Default|RemoveAllInstances _astrkwatergunsingleton_c))))

(event Custom|CallWithAuth
  (Networking|SwitchHasAuthority
    (:Authority
      (CallFunction|SpawnWaterVolume))))

(event EventTick
  (params (DeltaSeconds :type Float%20%28single-precision%29))
  (bind _returnvalue (* DeltaSeconds 1e+02))
  (bind _shotnum (Variables|Default|GetShotnum))
  (switch int _shotnum
    (:1
      (bind _returnvalue_2 (Class|Actor|GetOwnerController :!label _label))
      (bind _outactors (Actor|GetAllActorsOfClass "/Script/ShooterGame.NPCZoneVolume"))
      (bind _outhit (Collision|LineTraceForObjects (Transformation|GetActorLocation (Variables|/Script/Engine.PlayerController|GetPlayerCameraManager _returnvalue_2)) (+ (Transformation|GetActorLocation (Variables|/Script/Engine.PlayerController|GetPlayerCameraManager _returnvalue_2)) (* (Transformation|GetActorForwardVector (Variables|/Script/Engine.PlayerController|GetPlayerCameraManager _returnvalue_2)) 1e+05)) (Utilities|Array|MakeArray "ObjectTypeQuery9" "ObjectTypeQuery1" "ObjectTypeQuery2") false _outactors "ForOneFrame"))
      (switch int _shotnum
        (:1
          (Variables|Default|SetShot2Pos (.location _outhit))
          (Variables|Default|SetBoxDepth (Math|Float|Absolute(Float) (- (.z (Variables|Default|GetShot1Pos)) (.z (Variables|Default|GetShot2Pos))))))
        (:2
          (Variables|Default|SetShot3Pos (.location _outhit))))
      (CallFunction|RecalculateVars :!label _label_2)
      (CallFunction|UpdatePreview))
    (:2
      (goto _label))
    (:3
      ;[1 1 1] Handles Setting height/depth
      (Utilities|FlowControl|Sequence
        (:then_0
          (if (Variables|Default|GetIsHoldingRight)
            (if (Variables|Default|GetIsHolding1)
              (Variables|Default|SetBoxHeightOffset (+ (Variables|Default|GetBoxHeightOffset) _returnvalue))
              (elif (Variables|Default|GetIsHolding2)
                (Variables|Default|SetBoxHeightOffset (- (Variables|Default|GetBoxHeightOffset) _returnvalue))
                (elif (Variables|Default|GetIsHolding3)
                  (Variables|Default|SetBoxDepth (+ (Variables|Default|GetBoxDepth) _returnvalue))
                  (elif (Variables|Default|GetIsHolding4)
                    (Variables|Default|SetBoxDepth (- (Variables|Default|GetBoxDepth) _returnvalue))))))))
        (:then_1
          (goto _label_2))))))

(event EventEndPlay
  (params (EndPlayReason :type EEndPlayReason%20Enum :default "ActorDestroyed"))
  ;[1 1 1] Inits the preview box
  (Actor|DestroyActor (stale EventBeginPlay _returnvalue)))

(event EventBeginPlay
  (Utilities|SwitchNetAuthority
    (:PlayerServer
      _)
    (:Client
      _))
  (Utilities|FlowControl|Sequence
    (:then_0
      ;[1 1 1] Enables input
      (Input|EnableInput (Game|GetPlayerController 0)))
    (:then_1
      ;[1 1 1] Inits the preview box
      (bind _returnvalue (Game|SpawnActorfromClass "/Game/Mods/TRKWaterGun/WaterGun/TRKWaterVolumePreview_BP.TRKWaterVolumePreview_BP_C" (Math|Transform|MakeTransform (Math|Vector|MakeVector 0.0 0.0 -1e+05) "0, 0, 0" "1,1,1") false 0))
      (Variables|Default|SetPreviewCube (Variables|/Game/Mods/TRKWaterGun/WaterGun/TRKWaterVolumePreview_BP.TRKWaterVolumePreview_BP_C|GetStaticMesh1 _returnvalue))
      (Rendering|Material|SetMaterial (Variables|/Game/Mods/TRKWaterGun/WaterGun/TRKWaterVolumePreview_BP.TRKWaterVolumePreview_BP_C|GetStaticMesh1 _returnvalue) 0 "/Game/Mods/TRKWaterGun/WaterGun/Assets/M_TRKWaterVolumePreview.M_TRKWaterVolumePreview"))))

(event EventBPFiredWeapon
  (Utilities|SwitchNetAuthority
    (:PlayerServer
      _)
    (:Client
      _))
  (bind _returnvalue (Class|Actor|GetOwnerController))
  (bind _outactors (Actor|GetAllActorsOfClass "/Script/ShooterGame.NPCZoneVolume"))
  (bind (_outhit _returnvalue_2) (Collision|LineTraceForObjects (Transformation|GetActorLocation (Variables|/Script/Engine.PlayerController|GetPlayerCameraManager _returnvalue)) (+ (Transformation|GetActorLocation (Variables|/Script/Engine.PlayerController|GetPlayerCameraManager _returnvalue)) (* (Transformation|GetActorForwardVector (Variables|/Script/Engine.PlayerController|GetPlayerCameraManager _returnvalue)) 1e+05)) (Utilities|Array|MakeArray "ObjectTypeQuery9" "ObjectTypeQuery1" "ObjectTypeQuery2") false _outactors "ForOneFrame"))
  (if _returnvalue_2
    (if (Variables|Default|GetIsHoldingRight)
      ;[1 1 1] Removes box if right+left clicked
      (bind _astrkwatervolume_bp_c (Utilities|Casting|CastToTRKWaterVolume_BP (.hitactor _outhit))
        (:then
          (Default|RemoveBox _astrkwatervolume_bp_c))
        (:CastFailed
          (bind _asshooterplayercontroller (Utilities|Casting|CastToShooterPlayerController (Game|GetPlayerController 0)))
          (Class|ShooterPlayerController|ClientServerNotification :self _asshooterplayercontroller :MessageText "Failed to find Water Volume" :DisplayScale 1.0 :DisplayTime 2e+01)))
      (else
        ;[1 1 1] Set final position after shot and increment ShotNum
        (switch int (Variables|Default|GetShotnum)
          (:0
            (Variables|Default|SetShot1Pos (.location _outhit))
            (Variables|Default|SetShot2Pos (+ (.location _outhit) 1.0))
            (Variables|Default|SetShot3Pos (+ (.location _outhit) 1.0))
            (Variables|Default|SetBoxHeightOffset (.Z (Math|Vector|BreakVector (.location _outhit)))))
          (:1
            (Variables|Default|SetShot2Pos (.location _outhit))
            (Variables|Default|SetBoxDepth (Math|Float|Absolute(Float) (- (.z (Variables|Default|GetShot1Pos)) (.z (Variables|Default|GetShot2Pos))))))
          (:2
            (Variables|Default|SetShot3Pos (.location _outhit)))
          (:3
            _))
        (CallFunction|RecalculateVars)
        (CallFunction|UpdatePreview)
        (if (== (Variables|Default|GetShotnum) 3)
          ;[1 1 1] Spawn water and reset preview
          (Variables|Default|SetShotnum 0)
          (CallFunction|CallwithAuth)
          (Transformation|SetWorldLocation (Variables|Default|GetPreviewCube) "0, 0,-100000.000000" false)
          (else
            (Variables|Default|SetShotnum (+ (Variables|Default|GetShotnum) 1))))))
    (else
      (bind _asshooterplayercontroller_2 (Utilities|Casting|CastToShooterPlayerController _returnvalue))
      (Class|ShooterPlayerController|ClientServerNotification :self _asshooterplayercontroller_2 :MessageText "No point detected, try again" :DisplayScale 1.0 :DisplayTime 2.0))))

(event Input|KeyboardEvents|3
  ;[1 1 1] Sets input vars
  (:Pressed
    (Variables|Default|SetIsHolding3 true))
  (:Released
    (Variables|Default|SetIsHolding3 false)))

(event Input|KeyboardEvents|4
  ;[1 1 1] Sets input vars
  (:Pressed
    (Variables|Default|SetIsHolding4 true))
  (:Released
    (Variables|Default|SetIsHolding4 false)))

(event Input|KeyboardEvents|2
  ;[1 1 1] Sets input vars
  (:Pressed
    (Variables|Default|SetIsHolding2 true)
    ;[1 1 1] Deleting all objects from scene
    (if (Variables|Default|GetIsHoldingRight)
      (if (Variables|Default|GetIsHolding1)
        (if (== (Variables|Default|GetShotnum) 0)
          (CallFunction|DeleteAllVolumes)))))
  (:Released
    (Variables|Default|SetIsHolding2 false)))

(event Input|KeyboardEvents|1
  ;[1 1 1] Sets input vars
  (:Pressed
    (Variables|Default|SetIsHolding1 true))
  (:Released
    (Variables|Default|SetIsHolding1 false)))

(event Input|MouseEvents|RightMouseButton
  ;[1 1 1] Sets input vars
  (:Pressed
    (Variables|Default|SetIsHoldingRight true))
  (:Released
    (Variables|Default|SetIsHoldingRight false)))

(fn ConstructionScript
  (|CallParentFunction))

(fn UpdatePreview
  (Transformation|SetWorldTransform (Variables|Default|GetPreviewCube) (Math|Transform|MakeTransform (Variables|Default|GetBoxPos) (Math|Rotator|MakeRotator 0.0 (Variables|Default|GetBoxAngle) 0.0) (/ (Math|Vector|MakeVector (Variables|Default|GetBoxWidth) (Variables|Default|GetBoxLength) (Variables|Default|GetBoxDepth)) 256.0)) false))

(fn RecalculateVars
  (bind _boxdepth (Variables|Default|GetBoxDepth))
  (bind _boxheightoffset (Variables|Default|GetBoxHeightOffset))
  (bind _shot1pos (Variables|Default|GetShot1Pos))
  (bind _shot2pos (Variables|Default|GetShot2Pos))
  (bind _shot3pos (Variables|Default|GetShot3Pos))
  (bind _returnvalue (/ _boxdepth 2.0))
  (bind _returnvalue_2 (- (.y _shot2pos) (.y _shot1pos)))
  (bind _returnvalue_3 (- (.x _shot2pos) (.x _shot1pos)))
  (bind _returnvalue_4 (|(Ax+Bx)/2 (.x _shot1pos) (.x _shot2pos)))
  (bind _returnvalue_5 (|(Bx-Ax)*(Cy-Ay)-(By-Ay)*(Cx-Ax) (.x _shot2pos) (.x _shot1pos) (.y _shot3pos) (.y _shot1pos) (.y _shot2pos) (.x _shot3pos)))
  (bind _returnvalue_6 (- _boxheightoffset _returnvalue))
  (bind _returnvalue_7 (/ _returnvalue_2 _returnvalue_3))
  (bind _returnvalue_8 (/ _returnvalue_3 _returnvalue_2))
  (bind _returnvalue_9 (< _returnvalue_5 0.0))
  (bind _returnvalue_10 (* _returnvalue_8 -1.0))
  (bind _returnvalue_11 (|ABG*Ex+(Ay-ABG*Ax) _returnvalue_7 _returnvalue_4 (.y _shot1pos) (.x _shot1pos)))
  (bind _returnvalue_12 (|(Cy-Cx*G-Ay+Ax*ABG)/(ABG-G) (.y _shot3pos) (.x _shot3pos) _returnvalue_10 (.y _shot1pos) (.x _shot1pos) _returnvalue_7))
  (bind _returnvalue_13 (|ABG*Dx+(Ay-ABG*Ax) _returnvalue_7 _returnvalue_12 (.y _shot1pos) (.x _shot1pos)))
  (bind _returnvalue_14 (|CalcLength_2 _returnvalue_12 (.x _shot3pos) _returnvalue_13 (.y _shot3pos)))
  (bind _returnvalue_15 (|Ex+(Length/2)/Sqrt(1+Pow(G,2)) _returnvalue_4 _returnvalue_14 _returnvalue_10))
  (bind _returnvalue_16 (|Ex-(Length/2)/Sqrt(1+Pow(G,2)) _returnvalue_4 _returnvalue_14 _returnvalue_10))
  ;[1 1 1] AAAAAAAAAAAAAAAAAAAAAAAAAAAAAAAAAAAAAAAAAAAAAAAAAAAAAAAAAAAAAAAAAAAAAAAAAAAAAAAAAAAAAAAAAAAAAAAAAAAAAAAAAAAAAAAAAAAAAAAAAAAAAAAAAAAAAAAAAAAAAAAAAAAAAAAAAAAAAAAAAAAAAAA
  (Variables|Default|SetBoxWidth (|CalcWidth_2 (.x _shot2pos) (.x _shot1pos) (.y _shot2pos) (.y _shot1pos)))
  (Variables|Default|SetBoxLength _returnvalue_14)
  (if (< (.y _shot1pos) (.y _shot2pos))
    (if _returnvalue_9
      (Variables|Default|SetBoxPos (Math|Vector|MakeVector _returnvalue_15 (|G*xPos+(Ey-G*Ex) _returnvalue_10 _returnvalue_15 _returnvalue_11 _returnvalue_4) _returnvalue_6) :!label _label)
      (else
        (Variables|Default|SetBoxPos (Math|Vector|MakeVector _returnvalue_16 (|G*xPos+(Ey-G*Ex) _returnvalue_10 _returnvalue_16 _returnvalue_11 _returnvalue_4) _returnvalue_6) :!label _label_2)))
    (elif _returnvalue_9
      (goto _label_2)
      (else
        (goto _label))))
  (Variables|Default|SetBoxAngle (Class|KismetMathLibrary|DegAtan2 (- (.y _shot2pos) (.y _shot1pos)) (- (.x _shot2pos) (.x _shot1pos)))))

(fn SpawnWaterVolume
  (bind _outactors (Actor|GetAllActorsOfClass "/Game/Mods/TRKWaterGun/WaterGun/TRKWaterGunSingleton.TRKWaterGunSingleton_C"))
  (bind _astrkwatergunsingleton_c (Utilities|Casting|CastToTRKWaterGunSingleton (Utilities|Array|Get(acopy) _outactors)))
  (Default|AddInstance _astrkwatergunsingleton_c 0 (Utilities|Struct|MakeTRKWaterVolumeStruct (Variables|Default|GetBoxPos) (Math|Vector|MakeVector (Variables|Default|GetBoxWidth) (Variables|Default|GetBoxLength) (Variables|Default|GetBoxDepth)) (Variables|Default|GetBoxAngle) (Variables|Default|GetBoxHeightOffset) 0 (Utilities|Array|MakeArray 0))))